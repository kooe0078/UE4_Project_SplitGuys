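; BP_BulletSpawner is a moving emitter that repeatedly fires BP_BulletProjectile actors.
; Its construction script builds a two-point relative InterpToMovement path from the StartPosition, EndPosition and Duration variables.
; Tick feeds a Delay that throttles firing to roughly twice a second, each shot playing an explosion effect at the Arrow and spawning the projectile at a fixed world-X offset from it.
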(event EventTick
  (params (DeltaSeconds :type Float%20%28single-precision%29))
  (bind _arrow (Variables|Default|GetArrow))
  (bind _returnvalue (Transformation|GetWorldLocation _arrow))
  (Utilities|FlowControl|Delay 0.5)
  (Effects|SpawnEmitteratLocation "/Game/StarterContent/Particles/P_Explosion.P_Explosion" _returnvalue)
  (Game|SpawnActorfromClass "/Game/NewMaked/Objects/BP_BulletProjectile.BP_BulletProjectile_C" (Math|Conversions|ToTransform(Vector) (+ _returnvalue "100.000000, 0, 0")) "Undefined" 0 0))

(fn ConstructionScript
  (bind _interptomovement (Variables|Default|GetInterpToMovement))
  (Variables|/Script/Engine.InterpToMovementComponent|SetControlPoints _interptomovement (Utilities|Array|MakeArray (Utilities|Struct|MakeInterpControlPoint (Variables|Default|GetStartPosition) true) (Utilities|Struct|MakeInterpControlPoint (Variables|Default|GetEndPosition) true)))
  (Variables|/Script/Engine.InterpToMovementComponent|SetDuration _interptomovement (Variables|Default|Getduration)))