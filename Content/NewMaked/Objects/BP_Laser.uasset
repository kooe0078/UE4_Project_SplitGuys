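; BP_Laser is a laser object whose beam length follows whatever surface it points at.
; Each tick it passes its Laser component to LineTraceForLength, which runs a fixed-range Visibility trace along the component's forward vector, with debug drawing.
; On a hit, the component's world X scale is set from the hit distance with fixed thickness; on a miss, the previous scale remains.
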(event EventTick
  (params (DeltaSeconds :type Float%20%28single-precision%29))
  (for _array_element (Utilities|Array|MakeArray (Variables|Default|GetLaser))
    (CallFunction|LineTraceforLength _array_element)))

(fn ConstructionScript)

(fn LineTraceforLength
  (params (타깃 :type Scene%20Component%20Object%20Reference))
  (bind _laser (Variables|Default|GetLaser))
  (bind _returnvalue (Transformation|GetWorldLocation _laser))
  (bind (_outhit _returnvalue_2) (Collision|LineTraceByChannel _returnvalue (+ _returnvalue (* (Math|Vector|GetForwardVector _laser) 1e+03)) "TraceTypeQuery1" false 0 "ForOneFrame"))
  (if _returnvalue_2
    (Transformation|SetWorldScale3D 타깃 (Math|Vector|MakeVector (/ (Math|Vector|VectorLength (- (.Location (Collision|BreakHitResult _outhit)) (.TraceStart (Collision|BreakHitResult _outhit)))) 1e+01) 0.1 0.3))))